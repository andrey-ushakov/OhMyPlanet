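; BP_OMP_Pawn is a pawn that chooses the opening UI and manages a serial port connection during play.
; On BeginPlay it shows the BP_OMP_HUD widget if a save game exists, otherwise the BP_OMG_Start widget.
; It then opens the serial port, which it closes on EndPlay.
; A serial read-and-print chain is present but unconnected, so no incoming data is processed.
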(event `self.ReceiveBeginPlay`
  (`|ExecutionSequence`
    (:`then_0`
      (bind _returnvalue (`GameplayStatics.DoesSaveGameExist` (`self.DataSlot`)))
      (if _returnvalue
        (bind _returnvalue_2 (`|CreateWidget` "/Game/BP_OMP_HUD.BP_OMP_HUD_C"))
        (bind _output_get (set `self.Setup Reference` _returnvalue_2))
        (`UserWidget.AddToViewport` _output_get 0)
        (else
          (bind _returnvalue_3 (`|CreateWidget` "/Game/BP_OMG_Start.BP_OMG_Start_C"))
          (bind _output_get_2 (set `self.HUD Reference` _returnvalue_3))
          (`UserWidget.AddToViewport` _output_get_2 0))))
    (:`then_1`
      (`ThreadBP.OpenSerial` 6 115200))))

(event `self.ReceiveActorBeginOverlap`
  (params (OtherActor :type "Actor Object Reference")))

(event `self.ReceiveTick`
  (params (DeltaSeconds :type "Float (single-precision)")))

(event `self.ReceiveEndPlay`
  (params (EndPlayReason :type "EEndPlayReason Enum" :default "Destroyed"))
  (`ThreadBP.CloseSerial`))

(fn `UserConstructionScript`)